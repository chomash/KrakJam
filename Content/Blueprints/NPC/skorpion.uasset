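; Scorpion NPC interactable that opens the Scene_5 widget when the player uses it.
; A box trigger shows a text prompt and enables input while the player character overlaps it, and reverses both on exit.
; Pressing Interaction disables input, adds the widget, shows the mouse cursor, pauses the game after a short delay, then destroys the actor, making it one-use.
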(event `self.Box.OnComponentBeginOverlap`
  (params (OverlappedComponent :type "PrimitiveComponent Object Reference") (OtherActor :type "Actor Object Reference") (OtherComp :type "PrimitiveComponent Object Reference") (OtherBodyIndex :type Integer) (bFromSweep :type Boolean) (SweepResult :type "HitResult Structure (by ref)"))
  (cast `/Game/Player/PlayerCharacter` OtherActor)
  (`SceneComponent.SetVisibility` (`self.TextRender`) true false)
  (`self.EnableInput` (`GameplayStatics.GetPlayerController` 0)))

(event `self.Box.OnComponentEndOverlap`
  (params (OverlappedComponent :type "PrimitiveComponent Object Reference") (OtherActor :type "Actor Object Reference") (OtherComp :type "PrimitiveComponent Object Reference") (OtherBodyIndex :type Integer))
  (cast `/Game/Player/PlayerCharacter` OtherActor)
  (`SceneComponent.SetVisibility` (`self.TextRender`) false false)
  (`self.DisableInput` (`GameplayStatics.GetPlayerController` 0)))

(event `InputAction|Interaction`
  (params (Key :type "Key Structure"))
  (:`Pressed`
    (`self.DisableInput` null)
    (bind _returnvalue (`|CreateWidget` "/Game/Blueprints/Widgets/NPCs/Scene_5.Scene_5_C"))
    (`UserWidget.AddToViewport` _returnvalue 0)
    (set `PlayerController.bShowMouseCursor` true (`GameplayStatics.GetPlayerController` 0))
    (`KismetSystemLibrary.Delay` 0.2)
    (`GameplayStatics.SetGamePaused` true)
    (`self.K2_DestroyActor`)))

(fn `UserConstructionScript`)
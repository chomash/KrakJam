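; Snail_Pat is a one-shot interactable that lets the player pat a snail.
; A Box overlap by PlayerCharacter shows a TextRender and enables the actor's input, and leaving reverses both.
; Pressing Interaction sets the player's Objective text, adds a HeadPopUp widget, plays a sound and increments SnailsPatted on MyGameInstance, then the actor destroys itself.
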(event `self.Box.OnComponentBeginOverlap`
  (params (OverlappedComponent :type "PrimitiveComponent Object Reference") (OtherActor :type "Actor Object Reference") (OtherComp :type "PrimitiveComponent Object Reference") (OtherBodyIndex :type Integer) (bFromSweep :type Boolean) (SweepResult :type "HitResult Structure (by ref)"))
  (cast `/Game/Player/PlayerCharacter` OtherActor)
  (`SceneComponent.SetVisibility` (`self.TextRender`) true false)
  (`self.EnableInput` (`GameplayStatics.GetPlayerController` 0)))

(event `self.Box.OnComponentEndOverlap`
  (params (OverlappedComponent :type "PrimitiveComponent Object Reference") (OtherActor :type "Actor Object Reference") (OtherComp :type "PrimitiveComponent Object Reference") (OtherBodyIndex :type Integer))
  (cast `/Game/Player/PlayerCharacter` OtherActor)
  (`SceneComponent.SetVisibility` (`self.TextRender`) false false)
  (`self.DisableInput` (`GameplayStatics.GetPlayerController` 0)))

(event `InputAction|Interaction`
  (params (Key :type "Key Structure"))
  (:`Pressed`
    (`self.DisableInput` null)
    (bind _asplayer_character (cast `/Game/Player/PlayerCharacter` (`GameplayStatics.GetPlayerCharacter` 0)))
    (set `/Game/Player/PlayerCharacter.Objective` "pat pat pat" _asplayer_character)
    (bind _returnvalue (`|CreateWidget` "/Game/Blueprints/Widgets/HeadPopUp.HeadPopUp_C"))
    (`UserWidget.AddToViewport` _returnvalue 0)
    (`GameplayStatics.PlaySound2D` "/Game/Assets/Audio/glaskanie.glaskanie" 0.15 1.0 0.0 null null)
    (bind _asmy_game_instance (cast `/Game/Blueprints/MyGameInstance` (`GameplayStatics.GetGameInstance`)))
    (set `/Game/Blueprints/MyGameInstance.SnailsPatted` (+ (`/Game/Blueprints/MyGameInstance.SnailsPatted` _asmy_game_instance) 1) _asmy_game_instance)
    (`self.K2_DestroyActor`)))

(fn `UserConstructionScript`)
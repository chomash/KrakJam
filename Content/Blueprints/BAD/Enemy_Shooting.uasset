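; Enemy shooter actor that fires projectiles on a repeating timer and can be killed by damage.
; Shortly after BeginPlay it spawns an EnemyProjectile at each of three arrow components, passes on its Damage, then loops back through a one-second Delay.
; The player reference is cached at start but does not steer the shots.
; AnyDamage subtracts from Health and destroys the actor at zero or below.
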(event `self.ReceiveBeginPlay`
  ;[1 1 1] Shooting
  (bind _asplayer_character (cast `/Game/Player/PlayerCharacter` (`GameplayStatics.GetPlayerCharacter` 0)))
  (set `self.Player` _asplayer_character)
  (`KismetSystemLibrary.Delay` 0.5)
  (for _array_element (`|MakeArray` (`self.Arrow`) (`self.Arrow1`) (`self.Arrow3`)) :!label _label
    (bind _returnvalue (`|SpawnActorFromClass` "/Game/Blueprints/BAD/EnemyProjectile.EnemyProjectile_C" (`SceneComponent.K2_GetComponentToWorld` _array_element) "Undefined" "OverrideRootScale" null null))
    (set `/Game/Blueprints/BAD/EnemyProjectile.Damage` (`self.Damage`) _returnvalue)
    (`KismetSystemLibrary.Delay` 1.0)
    (goto _label)))

(event `self.ReceiveAnyDamage`
  (params (Damage :type "Float (single-precision)") (DamageType :type "DamageType Object Reference") (InstigatedBy :type "Controller Object Reference") (DamageCauser :type "Actor Object Reference"))
  ;[1 1 1] Taking Damage
  (bind _output_get (set `self.Health` (- (`self.Health`) Damage)))
  (if (<= _output_get 0.0)
    (`self.K2_DestroyActor`)))

(fn `UserConstructionScript`)